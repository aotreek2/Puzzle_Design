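; BP_WallManager is a Blueprint that builds a grid wall from instances on its Wall component.
; The AddWalls event clears existing instances, then loops over XSize columns and ZSize rows, adding one local-space instance per cell.
; XLength and ZHeight set the spacing along X and Z.
; The construction script is empty, so the grid is built only when AddWalls runs.
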(event Custom|Add%20Walls
  (Components|InstancedStaticMesh|ClearInstances (Variables|Default|GetWall))
  (for _index (range 0 (- (Variables|Default|GetXSize) 1))
    (for _index_2 (range 0 (- (Variables|Default|GetZSize) 1))
      (Components|InstancedStaticMesh|AddInstance (Variables|Default|GetWall) (Math|Transform|MakeTransform (Math|Vector|MakeVector (* _index (Variables|Default|GetXLength)) 0.0 (* _index_2 (Variables|Default|GetZHeight)))) false))))

(fn ConstructionScript)